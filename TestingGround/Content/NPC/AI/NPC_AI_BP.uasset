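; AI controller for NPCs that runs a patrol behavior tree and perceives actors.
; On BeginPlay it initializes the PatolData blackboard and starts the Patol behavior tree.
; Perception updates only print a debug message naming the pawn, sense class and perceived actor.
; FindPatrolRoute casts the pawn to PatrollingGuard and writes its first patrol point to the supplied blackboard's WayPoint key; this file never calls it.
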(event OnTargetPerceptionUpdated(AIPerception)
  (params (Actor :type Actor%20Object%20Reference) (Stimulus :type AI%20Stimulus%20Structure))
  (bind _returnvalue (Class|AIPerceptionSystem|GetSenseClassforStimulus Stimulus))
  (Development|PrintString (Utilities|String|Append (Utilities|GetObjectName (Pawn|GetControlledPawn)) "  Sees  " (Utilities|GetClassDisplayName _returnvalue) "  as  " (Utilities|GetObjectName Actor))))

(event EventBeginPlay
  (Class|AIController|UseBlackboard "/Game/NPC/AI/PatolData.PatolData")
  (AI|RunBehaviorTree "/Game/NPC/AI/Patol.Patol"))

(fn ConstructionScript)

(fn FindPatrolRoute
  (params (BlackBoard :type Blackboard%20Component%20Object%20Reference))
  (bind _aspatrolling_guard (Utilities|Casting|CastToPatrollingGuard (Pawn|GetControlledPawn)))
  (AI|Components|Blackboard|SetValueasObject BlackBoard (Utilities|Name|MakeLiteralName "WayPoint") (Utilities|Array|Get(acopy) (Variables|/Game/Trash/PatrollingGuard.PatrollingGuard_C|GetPatrolPoints _aspatrolling_guard))))