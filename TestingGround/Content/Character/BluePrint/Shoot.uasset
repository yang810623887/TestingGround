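; Behavior tree task that makes an AI-controlled TPCharacter aim and shoot at a target.
; On execute it sets the aiming and shooting flags and focuses the controller on the Target actor from the blackboard.
; It never finishes execution itself, so it runs until aborted, then clears both flags and focus and finishes the abort.
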(event EventReceiveExecuteAI
  (params (OwnerController :type AI%20Controller%20Object%20Reference) (ControlledPawn :type Pawn%20Object%20Reference))
  (bind _astpcharacter (Utilities|Casting|CastToTPCharacter ControlledPawn))
  (Variables|/Game/Character/TP_Character/TPCharacter.TPCharacter_C|SetAming _astpcharacter true)
  (Variables|/Game/Character/TP_Character/TPCharacter.TPCharacter_C|SetShooting _astpcharacter true)
  (AI|SetFocus OwnerController (AI|BehaviorTree|GetBlackboardValueasActor (Variables|Default|GetTarget))))

(event EventReceiveAbortAI
  (params (OwnerController :type AI%20Controller%20Object%20Reference) (ControlledPawn :type Pawn%20Object%20Reference))
  (bind _astpcharacter (Utilities|Casting|CastToTPCharacter ControlledPawn))
  (Variables|/Game/Character/TP_Character/TPCharacter.TPCharacter_C|SetAming _astpcharacter false)
  (Variables|/Game/Character/TP_Character/TPCharacter.TPCharacter_C|SetShooting _astpcharacter false)
  (AI|ClearFocus OwnerController)
  (Class|BTTaskBlueprintBase|FinishAbort))