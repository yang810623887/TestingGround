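; Game mode for an infinite terrain game that spawns chained terrain tiles and keeps the score.
; On BeginPlay it fills a nav mesh bounds volume pool, then runs a short startup loop that spawns tiles and, after a delay, calls TileConquered.
; Each tile receives the shared pool and supplies the attach location for the next tile's spawn.
; TileConquered increments the score, which a getter exposes.
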(event EventBeginPlay
  (Class|InfiniteTerrainGameMode|PopulateBoundsVolumePool)
  (for _index (range 0 3)
    (CallFunction|SpawnTile)
    (Utilities|FlowControl|Delay 0.2)
    (CallFunction|TileConquered)))

(fn ConstructionScript)

(fn SpawnTile
  (bind _returnvalue (Game|SpawnActorfromClass "/Game/Terrain/BP_Tile.BP_Tile_C" (Variables|Default|GetNext%20Tile%20Transform) "Undefined" 0 0))
  (Class|Tile|SetPool _returnvalue (Variables|Default|GetNavMeshBoundVolumePool))
  (bind _attach_transform (Default|GetAttachLocation _returnvalue))
  (Variables|Default|SetNext%20Tile%20Transform _attach_transform))

(fn TileConquered
  (Math|Integer|IncrementInt (Variables|Default|Getscore)))

(fn GetScorefromGameMode
  (return (Variables|Default|Getscore)))