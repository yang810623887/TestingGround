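; Behavior Tree task that advances a patrolling guard to its next waypoint.
; It reads the patrol points from the controlled PatrollingGuard pawn and writes the one at the blackboard Index into the WayPoint key.
; It then increments Index modulo the array length, so the route loops, and finishes with success.
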(event EventReceiveExecuteAI
  (params (OwnerController :type AI%20Controller%20Object%20Reference) (ControlledPawn :type Pawn%20Object%20Reference))
  (CallFunction|GetPatrolPoints ControlledPawn)
  (bind _newparam (CallFunction|SetNextWaypoint))
  (CallFunction|CycleIndex _newparam)
  (AI|BehaviorTree|FinishExecute true))

(fn GetPatrolPoints
  (params (Object :type Object%20Object%20Reference))
  (bind _aspatrolling_guard (Utilities|Casting|CastToPatrollingGuard Object))
  (Variables|Default|SetPatrolPoints (Variables|/Game/ThirdPersonCPP/Blueprints/PatrollingGuard.PatrollingGuard_C|GetPatrolPoints _aspatrolling_guard)))

(fn SetNextWaypoint
  (bind _index (Variables|Default|GetIndex))
  (bind _returnvalue (Class|BTFunctionLibrary|GetBlackboardValueasInt _index))
  (Class|BTFunctionLibrary|SetBlackboardValueasObject (Variables|Default|GetWayPoint) (Utilities|Array|Get(acopy) (Variables|Default|GetPatrolPoints) _returnvalue))
  (return _returnvalue))

(fn CycleIndex
  (params (Index :type Integer))
  (Class|BTFunctionLibrary|SetBlackboardValueasInt (Variables|Default|GetIndex) (Math|Integer|%(Integer) (+ Index 1) (Utilities|Array|Length (Variables|Default|GetPatrolPoints)))))