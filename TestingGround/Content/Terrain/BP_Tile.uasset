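; BP_Tile is one piece of an infinite terrain, with a barrier, trigger volumes and an arrow marking its attach transform.
; On BeginPlay it locks and calls PlaceActors to scatter randomly scaled cones.
; The player entering the locking volume opens the barrier (green, no collision); leaving re-locks it (red) and asks InfiniteTerrainGameMode to spawn another tile.
; The player entering the destroy volume destroys the tile.
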(event OnComponentBeginOverlap(LockingVolum)
  (params (OverlappedComponent :type Primitive%20Component%20Object%20Reference) (OtherActor :type Actor%20Object%20Reference) (OtherComp :type Primitive%20Component%20Object%20Reference) (OtherBodyIndex :type Integer) (bFromSweep :type Boolean) (SweepResult :type Hit%20Result%20Structure%20%28by%20ref%29))
  (Utilities|IsPlayerActor OtherActor)
  (CallFunction|UnLock))

(event OnComponentEndOverlap(LockingVolum)
  (params (OverlappedComponent :type Primitive%20Component%20Object%20Reference) (OtherActor :type Actor%20Object%20Reference) (OtherComp :type Primitive%20Component%20Object%20Reference) (OtherBodyIndex :type Integer))
  (Utilities|IsPlayerActor OtherActor)
  (CallFunction|Lock)
  (bind _asinfinite_terrain_game_mode (Utilities|Casting|CastToInfiniteTerrainGameMode (Game|GetGameMode)))
  (Default|SpawnTile _asinfinite_terrain_game_mode))

(event OnComponentBeginOverlap(DestoryVolum)
  (params (OverlappedComponent :type Primitive%20Component%20Object%20Reference) (OtherActor :type Actor%20Object%20Reference) (OtherComp :type Primitive%20Component%20Object%20Reference) (OtherBodyIndex :type Integer) (bFromSweep :type Boolean) (SweepResult :type Hit%20Result%20Structure%20%28by%20ref%29))
  (Utilities|IsPlayerActor OtherActor)
  (Actor|DestroyActor))

(event EventBeginPlay
  (CallFunction|Lock)
  (Class|Tile|PlaceActors "/Game/Terrain/props/Cone.Cone_C" 1 20 5e+02 0.1 2.0))

(fn ConstructionScript)

(fn GetAttachLocation
  (return (Transformation|GetWorldTransform (Variables|Default|GetArrow))))

(fn UnLock
  (Collision|SetCollisionEnabled (Variables|Default|GetBarrier) "NoCollision")
  (Rendering|Material|SetMaterial (Variables|Default|GetBarrier) 0 "/Game/Terrain/MI_Barrier_Green.MI_Barrier_Green"))

(fn Lock
  (Collision|SetCollisionEnabled (Variables|Default|GetBarrier) "QueryAndPhysics")
  (Rendering|Material|SetMaterial (Variables|Default|GetBarrier) 0 "/Game/Terrain/MI_Barrier_Red.MI_Barrier_Red"))